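; BP_Sagar is the player character, with first-person-style camera-relative movement, jumping, object interaction, ladder climbing and a beer-case carry that slows walking.
; Looking triggers camera line traces for BPI_Interactable actors to update HUD prompts, and interact repeats the trace to message them.
; Ladders switch movement mode to None and move the actor manually between endpoints.
; WB_Game_UI handles phone navigation, pause and the delayed game-over after being caught; phone mode blocks move and look.
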(event Custom|Player%20started%20holding%20beer%20bottles
  (params (Beer%20Case :type Beer%20Bottles%20Object%20Reference))
  ;[1 1 1] Beer Bottles mesh
  (Variables|Default|SetBeer%20Case Beer%20Case)
  (Variables|/Script/Engine.CharacterMovementComponent|SetMaxWalkSpeed (Variables|Character|GetCharacterMovement) 4e+02)
  (Variables|Default|SetHas%20Beer%20Bottles? true))

(event Custom|Player%20has%20left%20Bottles
  ;[1 1 1] Beer Bottles mesh
  (Actor|DestroyActor (Variables|Default|GetBeer%20Case))
  (Variables|Default|SetBeer%20Case 0)
  (Variables|/Script/Engine.CharacterMovementComponent|SetMaxWalkSpeed (Variables|Character|GetCharacterMovement) 6e+02)
  (Variables|Default|SetHas%20Beer%20Bottles? false))

(event Custom|Sagar%20Caught
  (bind _returnvalue (Game|GetPlayerController 0))
  (bind _gamehud (Variables|Default|GetGameHud))
  (Pawn|Components|CharacterMovement|DisableMovement (Variables|Character|GetCharacterMovement))
  (Variables|Default|Setb_Caught true)
  (Audio|PlaySound2D "/Game/Audio/Effects/Sagar_s_sudden_suppai.Sagar_s_sudden_suppai" 1.0 1.0 0.0 0 0)
  (Utilities|FlowControl|Delay 8.5)
  (Audio|PlaySound2D "/Game/Audio/Effects/Bonk_Sound_Effect.Bonk_Sound_Effect" 1.0 1.0 0.0 0 0)
  (Utilities|FlowControl|Delay 2.0)
  (Default|GameOver _gamehud)
  (Input|SetInputModeUIOnly _returnvalue _gamehud "DoNotLock" false)
  (Variables|/Script/Engine.PlayerController|SetbShowMouseCursor _returnvalue true))

(event Custom|Trace%20for%20Interactables
  (bind _camera (Variables|Default|GetCamera))
  (bind _returnvalue (Transformation|GetWorldLocation _camera))
  ;[1 1 1] Ladder Component
  (bind _outhits (Collision|MultiLineTraceByChannel _returnvalue (+ _returnvalue (* (Math|Vector|GetForwardVector _camera) (Variables|Default|GetInteractable%20Distance))) "TraceTypeQuery1" false 0 "None"))
  (Variables|Default|SetCan%20Interact%20with false)
  (for _array_element _outhits
    (if (Math|Boolean|ANDBoolean (not (Variables|Default|GetOnLadder)) (.bBlockingHit (Collision|BreakHitResult _array_element)) (Utilities|DoesObjectImplementInterface (.HitActor (Collision|BreakHitResult _array_element)) "/Game/Game_Files/BPI_Interactable.BPI_Interactable_C"))
      (Variables|Default|SetCan%20Interact%20with true)
      (bind _item_name (Class|BPIInteractable|GetInteractableName(Message) (.HitActor (Collision|BreakHitResult _array_element))))
      (Variables|Default|SetInteractable%20Name _item_name)))
  (Default|CanInteractWObject (Variables|Default|GetGameHud) (Variables|Default|GetCan%20Interact%20with) (Variables|Default|GetInteractable%20Name)))

(event Custom|Interact%20With%20Object
  (bind _camera (Variables|Default|GetCamera))
  (bind _returnvalue (Transformation|GetWorldLocation _camera))
  ;[1 1 1] Ladder Component
  (bind _outhits (Collision|MultiLineTraceByChannel _returnvalue (+ _returnvalue (* (Math|Vector|GetForwardVector _camera) (Variables|Default|GetInteractable%20Distance))) "TraceTypeQuery1" false 0 "None"))
  (for _array_element _outhits
    (if (Math|Boolean|ANDBoolean (not (Variables|Default|GetOnLadder)) (.bBlockingHit (Collision|BreakHitResult _array_element)) (Utilities|DoesObjectImplementInterface (.HitActor (Collision|BreakHitResult _array_element)) "/Game/Game_Files/BPI_Interactable.BPI_Interactable_C"))
      (Class|BPIInteractable|TryInteract(Message) (.HitActor (Collision|BreakHitResult _array_element)) self))))

(event Custom|Ladder%20Movement
  (params (Movement :type Float%20%28double-precision%29))
  (if (or (and (> Movement 0.0) (Variables|Default|GetLadder%20Bottom)) (and (< Movement 0.0) (not (Variables|Default|GetLadder%20Bottom))))
    (Transformation|SetActorRelativeLocation (+ (Transformation|GetActorLocation) (* Movement (Variables|Default|GetLadder%20Climbing%20Speed))))
    (if (< (Math|Vector|Distance(Vector) (Transformation|GetActorLocation) (Variables|Default|GetLadder%20Bottom%20Point)) 4.0)
      (Default|UnMountfromLadder self)
      (elif (< (Math|Vector|Distance(Vector) (Transformation|GetActorLocation) (Variables|Default|GetLadder%20Top%20Point)) 4.0)
        (Default|UnMountfromLadder self)))))

(event Input|EnhancedActionEvents|EnhancedInputActionIA_Move
  (params (ActionValue :type Vector%202D%20Structure) (ElapsedSeconds :type Float%20%28double-precision%29) (TriggeredSeconds :type Float%20%28double-precision%29) (InputAction :type Input%20Action%20Object%20Reference :default "/Game/Game_Files/Player/IA_Move.IA_Move"))
  (bind (_x _y) (Math|Vector2D|BreakVector2D ActionValue))
  ;[1 1 1] Adding Inputs
  (if (not (Variables|Default|Getb_Phone%20Mode))
    (if (Variables|Default|GetOnLadder)
      (CallFunction|LadderMovement _x)
      (else
        (Pawn|Input|AddMovementInput (Math|Vector|GetForwardVector (Variables|Default|GetCamera)) _x false)
        (Pawn|Input|AddMovementInput (Math|Vector|GetRightVector (Variables|Default|GetCamera)) _y false)))))

(event Input|EnhancedActionEvents|EnhancedInputActionIA_Look
  (params (ActionValue :type Vector%202D%20Structure) (ElapsedSeconds :type Float%20%28double-precision%29) (TriggeredSeconds :type Float%20%28double-precision%29) (InputAction :type Input%20Action%20Object%20Reference :default "/Game/Game_Files/Player/IA_Look.IA_Look"))
  (bind (_x _y) (Math|Vector2D|BreakVector2D ActionValue))
  (bind _mouse_sensitivity (Variables|Default|GetMouse%20Sensitivity))
  ;[1 1 1] Adding Inputs
  (if (not (or (Variables|Default|Getb_Phone%20Mode) (Variables|Default|Getb_Caught)))
    (Pawn|Input|AddControllerYawInput (* _mouse_sensitivity _x))
    (Pawn|Input|AddControllerPitchInput (Math|Float|MapRangeClamped (* _y _mouse_sensitivity) -1.0 1.0 1.0 -1.0))
    (CallFunction|TraceforInteractables)))

(event Input|EnhancedActionEvents|EnhancedInputActionIA_Phone_InteractRight
  (params (ActionValue :type Boolean) (ElapsedSeconds :type Float%20%28double-precision%29) (TriggeredSeconds :type Float%20%28double-precision%29) (InputAction :type Input%20Action%20Object%20Reference :default "/Game/Game_Files/Player/IA_Phone_InteractRight.IA_Phone_InteractRight"))
  (Class|BPIPhone|PhoneInteract(Message) (Variables|Default|GetGameHud) "NewEnumerator1"))

(event Input|EnhancedActionEvents|EnhancedInputActionIA_Phone_InteractUp
  (params (ActionValue :type Boolean) (ElapsedSeconds :type Float%20%28double-precision%29) (TriggeredSeconds :type Float%20%28double-precision%29) (InputAction :type Input%20Action%20Object%20Reference :default "/Game/Game_Files/Player/IA_Phone_InteractUp.IA_Phone_InteractUp"))
  (Class|BPIPhone|PhoneInteract(Message) (Variables|Default|GetGameHud) "NewEnumerator2"))

(event Input|EnhancedActionEvents|EnhancedInputActionIA_Phone_InteractSelect
  (params (ActionValue :type Boolean) (ElapsedSeconds :type Float%20%28double-precision%29) (TriggeredSeconds :type Float%20%28double-precision%29) (InputAction :type Input%20Action%20Object%20Reference :default "/Game/Game_Files/Player/IA_Phone_InteractSelect.IA_Phone_InteractSelect"))
  (Class|BPIPhone|PhoneInteract(Message) (Variables|Default|GetGameHud) "NewEnumerator4"))

(event Input|EnhancedActionEvents|EnhancedInputActionIA_Jump
  (params (ActionValue :type Boolean) (ElapsedSeconds :type Float%20%28double-precision%29) (TriggeredSeconds :type Float%20%28double-precision%29) (InputAction :type Input%20Action%20Object%20Reference :default "/Game/Game_Files/Player/IA_Jump.IA_Jump"))
  ;[1 1 1] Jumping
  (Character|Jump))

(event Input|EnhancedActionEvents|EnhancedInputActionIA_Pickup
  (params (ActionValue :type Boolean) (ElapsedSeconds :type Float%20%28double-precision%29) (TriggeredSeconds :type Float%20%28double-precision%29) (InputAction :type Input%20Action%20Object%20Reference :default "/Game/Game_Files/Player/IA_Pickup.IA_Pickup"))
  ;[1 1 1] Pickup
  (:Started
    (Variables|Default|SetPickUpPressed true))
  (:Completed
    (Variables|Default|SetPickUpPressed false)))

(event Input|EnhancedActionEvents|EnhancedInputActionIA_Interact
  (params (ActionValue :type Boolean) (ElapsedSeconds :type Float%20%28double-precision%29) (TriggeredSeconds :type Float%20%28double-precision%29) (InputAction :type Input%20Action%20Object%20Reference :default "/Game/Game_Files/Player/IA_Interact.IA_Interact"))
  ;[1 1 1] Interacting
  (:Started
    (CallFunction|InteractwithObject)))

(event Input|EnhancedActionEvents|EnhancedInputActionIA_Pause
  (params (ActionValue :type Boolean) (ElapsedSeconds :type Float%20%28double-precision%29) (TriggeredSeconds :type Float%20%28double-precision%29) (InputAction :type Input%20Action%20Object%20Reference :default "/Game/Game_Files/Player/IA_Pause.IA_Pause"))
  ;[1 1 1] Pause Menu
  (:Started
    (Utilities|FlowControl|FlipFlop
      (:A
        (Default|ActivatePanel/Animation (Variables|Default|GetGameHud) "NewEnumerator6")
        (Game|SetGamePaused true))
      (:B
        (Default|ActivatePanel/Animation (Variables|Default|GetGameHud) "NewEnumerator0")
        (Game|SetGamePaused false)))))

(event Input|EnhancedActionEvents|EnhancedInputActionIA_Phone
  (params (ActionValue :type Boolean) (ElapsedSeconds :type Float%20%28double-precision%29) (TriggeredSeconds :type Float%20%28double-precision%29) (InputAction :type Input%20Action%20Object%20Reference :default "/Game/Game_Files/Player/IA_Phone.IA_Phone"))
  ;[1 1 1] Bring Up Phone
  (:Started
    (bind _isa (Utilities|FlowControl|FlipFlop)
      (:A
        _)
      (:B
        _))
    (bind _output_get (Variables|Default|Setb_Phone%20Mode _isa))
    (Default|PhoneMode (Variables|Default|GetGameHud) _output_get)))

(event Input|EnhancedActionEvents|EnhancedInputActionIA_Phone_InteractDown
  (params (ActionValue :type Boolean) (ElapsedSeconds :type Float%20%28double-precision%29) (TriggeredSeconds :type Float%20%28double-precision%29) (InputAction :type Input%20Action%20Object%20Reference :default "/Game/Game_Files/Player/IA_Phone_InteractDown.IA_Phone_InteractDown"))
  (Class|BPIPhone|PhoneInteract(Message) (Variables|Default|GetGameHud) "NewEnumerator3"))

(event Input|EnhancedActionEvents|EnhancedInputActionIA_Phone_InteractLeft
  (params (ActionValue :type Boolean) (ElapsedSeconds :type Float%20%28double-precision%29) (TriggeredSeconds :type Float%20%28double-precision%29) (InputAction :type Input%20Action%20Object%20Reference :default "/Game/Game_Files/Player/IA_Phone_InteractLeft.IA_Phone_InteractLeft"))
  (Class|BPIPhone|PhoneInteract(Message) (Variables|Default|GetGameHud) "NewEnumerator0"))

(event EventBeginPlay
  ;[1 1 1] Binding Input Actions
  (Input|AddMappingContext (PlayerController|LocalPlayerSubsystems|GetEnhancedInputLocalPlayerSubsystem (Game|GetPlayerController 0)) "/Game/Game_Files/Player/Player_Input_System.Player_Input_System" 0 "(bIgnoreAllPressedKeysUntilRelease=True,bForceImmediately=False,bNotifyUserSettings=False)")
  (bind _returnvalue (UserInterface|CreateWidget "/Game/UIAssets/WB_Game_UI.WB_Game_UI_C"))
  (bind _output_get (Variables|Default|SetGameHud _returnvalue))
  (UserInterface|Viewport|AddtoViewport _output_get 0))

(event EventCCTVPage
  (params (Active :type Boolean) (Active%20Camera%20Index :type Integer))
  (Default|CallCCTVMode Active Active%20Camera%20Index))

(event EventMounttoLadder
  (params (Bottom%20Point :type Vector :default "0, 0, 0") (Top%20Point :type Vector :default "0, 0, 0"))
  (bind _returnvalue (Transformation|GetActorLocation))
  (Variables|Default|SetLadder%20Bottom%20Point Bottom%20Point)
  (Variables|Default|SetLadder%20Top%20Point Top%20Point)
  (Pawn|Components|CharacterMovement|SetMovementMode (Variables|Character|GetCharacterMovement) "MOVE_None" 0)
  (Variables|Default|SetLadder%20Bottom (< (Math|Vector|Distance(Vector) _returnvalue (Variables|Default|GetLadder%20Bottom%20Point)) (Math|Vector|Distance(Vector) _returnvalue (Variables|Default|GetLadder%20Top%20Point))))
  (Transformation|SetActorLocation (Math|Vector|SelectVector (Variables|Default|GetLadder%20Bottom%20Point) (Variables|Default|GetLadder%20Top%20Point) (< (Math|Vector|Distance(Vector) _returnvalue (Variables|Default|GetLadder%20Bottom%20Point)) (Math|Vector|Distance(Vector) _returnvalue (Variables|Default|GetLadder%20Top%20Point)))) false false)
  (Variables|Default|SetOnLadder true)
  (Default|CanInteractWObject (Variables|Default|GetGameHud) false))

(event EventUnMountfromLadder
  (Transformation|AddActorWorldOffset "10.000000,0.000000,0.000000")
  (Pawn|Components|CharacterMovement|SetMovementMode (Variables|Character|GetCharacterMovement) "MOVE_Walking" 0)
  (Variables|Default|SetOnLadder false))

(fn ConstructionScript)

(fn GetInteractableName
  (return ""))