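; BP_Nandini_Pawn is the AI enemy character that catches the player, BP_Sagar, through its Kill overlap component.
; The first overlap calls SagarCaught, starts a surprised montage, disables movement and unpossesses the AI controller, then plays a sword attack after a timed delay.
; A separate PlayHittingMontage event plays that attack and opens MainMenu if its Sagar reference is valid.
; Sound playback logic is present but disconnected.
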(event OnComponentBeginOverlap(Kill)
  (params (OverlappedComponent :type Primitive%20Component%20Object%20Reference) (OtherActor :type Actor%20Object%20Reference) (OtherComp :type Primitive%20Component%20Object%20Reference) (OtherBodyIndex :type Integer) (bFromSweep :type Boolean) (SweepResult :type Hit%20Result%20Structure%20%28by%20ref%29))
  (bind _returnvalue (AI|GetAIController 0))
  (bind _asbp_sagar (Utilities|Casting|CastToBP_Sagar OtherActor))
  (Utilities|FlowControl|DoOnce false
    (:Completed
      (Default|SagarCaught _asbp_sagar)
      (Animation|Montage|PlayMontage (Variables|Character|GetMesh) "/Game/Game_Files/AI/Anims/Surprised_Montage.Surprised_Montage"
        (:then
          (Pawn|Components|CharacterMovement|DisableMovement (Variables|Character|GetCharacterMovement))
          (Input|DisableInput _returnvalue 0)
          (Pawn|UnPossess _returnvalue)
          (Variables|Default|SetbUseControllerRotationPitch false)
          (Variables|Default|SetbUseControllerRotationRoll false)
          (Variables|Default|SetbUseControllerRotationYaw false)
          (Utilities|FlowControl|Delay 8.5)
          (Animation|Montage|PlayMontage (Variables|Character|GetMesh) "/Game/Game_Files/AI/Anims/Great_Sword_Attack_Montage.Great_Sword_Attack_Montage"))))))

(event Custom|Play%20Hitting%20%20Montage
  (Animation|Montage|PlayMontage (Variables|Character|GetMesh) "/Game/Game_Files/AI/Anims/Great_Sword_Attack_Montage.Great_Sword_Attack_Montage"
    (:OnCompleted
      (Utilities|IsValid (Variables|Default|GetAs%20BP%20Sagar)
        (:Is%20Valid
          (Utilities|FlowControl|Delay 0.2)
          (Game|OpenLevel(byName) "MainMenu"))))))

(event EventTick
  (params (DeltaSeconds :type Float%20%28single-precision%29)))

(event EventBeginPlay)

(fn ConstructionScript)