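; Interactable fridge with an animated door that doubles as the beer-bottle task point for BP_Sagar.
; Overlap by Sagar or Nandini caches the actor and highlights the fridge through custom depth.
; TryInteract toggles the door on a timeline with sound.
; When the fridge is open, it also stores Sagar's bottles or spawns bottles attached to Sagar, depending on JOG_GM's current level, then reports the task complete.
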(event OnComponentBeginOverlap(FridgeCollision)
  (params (OverlappedComponent :type Primitive%20Component%20Object%20Reference) (OtherActor :type Actor%20Object%20Reference) (OtherComp :type Primitive%20Component%20Object%20Reference) (OtherBodyIndex :type Integer) (bFromSweep :type Boolean) (SweepResult :type Hit%20Result%20Structure%20%28by%20ref%29))
  (Variables|Default|SetCan%20interact (CallFunction|CastChecker OtherActor false))
  (Rendering|SetRenderCustomDepth (Variables|Default|GetFridgeBase) (Variables|Default|GetCan%20interact)))

(event OnComponentEndOverlap(FridgeCollision)
  (params (OverlappedComponent :type Primitive%20Component%20Object%20Reference) (OtherActor :type Actor%20Object%20Reference) (OtherComp :type Primitive%20Component%20Object%20Reference) (OtherBodyIndex :type Integer))
  (Variables|Default|SetCan%20interact (CallFunction|CastChecker OtherActor true))
  (Rendering|SetRenderCustomDepth (Variables|Default|GetFridgeBase) (Variables|Default|GetCan%20interact)))

(event EventTryInteract
  (params (Actor%20 :type Actor%20Object%20Reference))
  (bind _other_actor (Variables|Default|GetOther%20Actor))
  (bind _other_actor_2 (Variables|Default|GetOther%20Actor))
  (bind _asbp_sagar (Utilities|Casting|CastToBP_Sagar _other_actor_2))
  (Utilities|FlowControl|Sequence
    (:then_0
      (switch Utilities|FlowControl|Switch|SwitchonETimelineDirection (Variables|Default|GetDirection)
        (:Forward
          (bind (_direction _time_to_open) (Timeline|OneFridgeGate Reverse)
            (:Update
              (Transformation|SetRelativeLocationAndRotation (Variables|Default|GetFridge%20Gate) (Math|Vector|Lerp(Vector) "0, 0, 0" "0.000000,50.000000,0.000000" _time_to_open) (Math|Rotator|Lerp(Rotator) "0, 0, 0" "0.000000,-90.000000,0.000000" _time_to_open) false false)
              (Utilities|FlowControl|DoOnce false :!label _label
                (:Completed
                  (Audio|PlaySoundatLocation "/Game/Intractable/Audio/Cupbord2.Cupbord2" (Transformation|GetActorLocation) "0, 0, 0" 0.3 1.0 0.0 0 0 0 0))))
            (:Finished
              (bind _output_get (Variables|Default|SetDirection _direction))
              (switch Utilities|FlowControl|Switch|SwitchonETimelineDirection _output_get
                (:Forward
                  (Variables|Default|SetFridge%20Open? true)
                  (goto _label Reset))
                (:Backward
                  (Variables|Default|SetFridge%20Open? false)
                  (goto _label Reset))))))
        (:Backward
          (Timeline|OneFridgeGate Play))))
    (:then_1
      ;[1 1 1] Checking Current Level
      (if (Utilities|Enum|Equal(Enum) (Variables|/Game/Game_Files/JOG_GM.JOG_GM_C|GetCurrent%20Level (.AsJOG%20GM (Utilities|Casting|CastToJOG_GM (Game|GetGameMode)))) "NewEnumerator1")
        ;[1 1 1] Checking if player has beer bottles
        (Utilities|IsValid _other_actor
          (:Is%20Valid
            (if (and (Variables|/Game/Game_Files/Player/BP_Sagar.BP_Sagar_C|GetHas%20Beer%20Bottles? (.AsBP%20Sagar (Utilities|Casting|CastToBP_Sagar _other_actor))) (Variables|Default|GetFridge%20Open?))
              ;[1 1 1] Handling Internal Beer case visiblity, Destroying the player held character and updating the char speed
              (Rendering|SetVisibility (Variables|Default|GetBeer%20Case) true false)
              (Default|PlayerHasLeftBottles (.AsBP%20Sagar (Utilities|Casting|CastToBP_Sagar (Variables|Default|GetOther%20Actor))))
              ;[1 1 1] Updating The Gm
              (Default|TaskCompleted (.AsJOG%20GM (Utilities|Casting|CastToJOG_GM (Game|GetGameMode))))
              (Timeline|OneFridgeGate Reverse)))
          (:Is%20Not%20Valid
            ;[1 1 1] Checking if current level is taking bottles
            (if (and (Utilities|Enum|Equal(Enum) (Variables|/Game/Game_Files/JOG_GM.JOG_GM_C|GetCurrent%20Level (.AsJOG%20GM (Utilities|Casting|CastToJOG_GM (Game|GetGameMode)))) "NewEnumerator3") (Variables|Default|GetFridge%20Open?)) :!label _label_2
              ;[1 1 1] Making sure player doesnt have bottles already
              (Utilities|IsValid _asbp_sagar
                (:Is%20Valid
                  (if (not (Variables|/Game/Game_Files/Player/BP_Sagar.BP_Sagar_C|GetHas%20Beer%20Bottles? _asbp_sagar))
                    ;[1 1 1] Disable beer case and spawn new actor and attach it to our main character
                    (Rendering|SetVisibility (Variables|Default|GetBeer%20Case) false false)
                    (bind _returnvalue (Game|SpawnActorfromClass "/Game/Intractable/BeerBottles.BeerBottles_C" (Math|Transform|MakeTransform "0, 0, 0" "0, 0, 0" "1.000000,1.000000,1.000000") "AlwaysSpawn" "OverrideRootScale" 0 0))
                    (Default|PlayerStartedHoldingBeerBottles (.AsBP%20Sagar (Utilities|Casting|CastToBP_Sagar (Variables|Default|GetOther%20Actor))) _returnvalue)
                    (Transformation|AttachComponentToComponent _returnvalue (Variables|/Game/Game_Files/Player/BP_Sagar.BP_Sagar_C|GetBeer%20Bottle%20Holder (.AsBP%20Sagar (Utilities|Casting|CastToBP_Sagar (Variables|Default|GetOther%20Actor)))) "None" "SnapToTarget" "SnapToTarget" "SnapToTarget" false)
                    ;[1 1 1] Updating Player and GM
                    (Default|TaskCompleted (.AsJOG%20GM (Utilities|Casting|CastToJOG_GM (Game|GetGameMode))))))))))
        (else
          (goto _label_2))))))

(event Collision|EventActorBeginOverlap
  (params (OtherActor :type Actor%20Object%20Reference)))

(fn ConstructionScript)

(fn CastChecker
  (params (Object :type Actor%20Object%20Reference) (Exit? :type Boolean))
  (Variables|Default|SetOther%20Actor Object)
  (if (or (.bSuccess (Utilities|Casting|CastToBP_Sagar Object)) (.bSuccess (Utilities|Casting|CastToBP_Nandini_Pawn Object)))
    (if Exit?
      (Variables|Default|SetOther%20Actor 0)
      (return false)
      (else
        (return true)))
    (else
      (Variables|Default|SetOther%20Actor 0))))

(fn GetInteractableName
  (return "Fridge"))