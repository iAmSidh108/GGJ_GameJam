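; BP_CCTV is a security camera actor that feeds its view into a render target through a scene capture component.
; On BeginPlay it assigns the texture target and binds to the CCTV mode event on the player's BP_Sagar pawn.
; When the mode turns on, a looping timer captures the scene every fraction of a second instead of continuously; turning it off pauses the timer.
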(event Custom|CCTV%20Feed%20Active
  (params (Active? :type Boolean))
  (bind _output_get (Variables|Default|SetActive? Active?))
  (if _output_get
    (bind _returnvalue (Utilities|Time|SetTimerbyFunctionName 0 "Capture Scene" 0.05 true))
    (Variables|Default|SetTimer%20Function _returnvalue)
    (else
      (Utilities|Time|PauseTimerbyHandle (Variables|Default|GetTimer%20Function)))))

(event Custom|Capture%20Scene
  (Rendering|SceneCapture|CaptureScene (Variables|Default|GetSceneCaptureComponent2D) :!class /Script/Engine.SceneCaptureComponent2D))

(event EventBeginPlay
  (Variables|/Script/Engine.SceneCaptureComponent2D|SetTextureTarget (Variables|Default|GetSceneCaptureComponent2D) (Variables|Default|GetTexture%20Target))
  (EventDispatchers|BindEventtoCCTVMode (.AsBP%20Sagar (Utilities|Casting|CastToBP_Sagar (Pawn|GetControlledPawn (Game|GetPlayerController 0)))) (delegate Custom|CCTV%20Feed%20Active)))

(fn ConstructionScript)