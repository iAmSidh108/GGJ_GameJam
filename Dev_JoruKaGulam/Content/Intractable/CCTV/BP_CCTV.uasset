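; CCTV camera actor that feeds its view into a render target while the player watches that camera.
; On BeginPlay it assigns the target to its scene capture component and binds to the BP_Sagar pawn's CCTV mode event.
; When the feed is active and the index matches its own, a looping timer triggers manual captures at roughly 12 fps.
; Otherwise it clears the timer, so unselected cameras stop timed captures.
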(event Custom|CCTV%20Feed%20Active
  (params (Active? :type Boolean) (Active%20CCTV%20Index :type Integer))
  (bind _output_get (Variables|Default|SetActive? Active?))
  (if (and _output_get (== Active%20CCTV%20Index (Variables|Default|GetCamera%20Index)))
    (bind _returnvalue (Utilities|Time|SetTimerbyFunctionName 0 "Capture Scene" 0.083 true))
    (Variables|Default|SetTimer%20Function _returnvalue)
    (Development|PrintString (Utilities|String|Append "Activating Camera : " (Utilities|String|ToString(Integer) (Variables|Default|GetCamera%20Index))))
    (else
      (Utilities|Time|ClearandInvalidateTimerbyHandle (Variables|Default|GetTimer%20Function)))))

(event Custom|Capture%20Scene
  (Rendering|SceneCapture|CaptureScene (Variables|Default|GetSceneCaptureComponent2D) :!class /Script/Engine.SceneCaptureComponent2D))

(event EventBeginPlay
  (Variables|/Script/Engine.SceneCaptureComponent2D|SetTextureTarget (Variables|Default|GetSceneCaptureComponent2D) (Variables|Default|GetTexture%20Target))
  (EventDispatchers|BindEventtoCCTVMode (.AsBP%20Sagar (Utilities|Casting|CastToBP_Sagar (Pawn|GetControlledPawn (Game|GetPlayerController 0)))) (delegate Custom|CCTV%20Feed%20Active)))

(fn ConstructionScript)