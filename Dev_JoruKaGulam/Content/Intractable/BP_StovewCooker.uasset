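; Interactable rice cooker that makes a one-time noise event detectable by AI.
; TryInteract passes through a DoOnce, starts the audio, then after a delay reports a loud noise at the cooker's location.
; A BP_Nandini_Pawn entering the collider stops the audio, without cancelling the pending noise report.
; A CastChecker helper validates Sagar or Nandini actors but is not called in this event graph.
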(event OnComponentBeginOverlap(Collider)
  (params (OverlappedComponent :type Primitive%20Component%20Object%20Reference) (OtherActor :type Actor%20Object%20Reference) (OtherComp :type Primitive%20Component%20Object%20Reference) (OtherBodyIndex :type Integer) (bFromSweep :type Boolean) (SweepResult :type Hit%20Result%20Structure%20%28by%20ref%29))
  (Utilities|Casting|CastToBP_Nandini_Pawn OtherActor)
  (Audio|Components|Audio|Stop (Variables|Default|GetAudio)))

(event EventTryInteract
  (Development|PrintString "Trying to interact with Cooker")
  (Utilities|FlowControl|DoOnce false
    (:Completed
      (Audio|Components|Audio|Play (Variables|Default|GetAudio) 0.0)
      (Utilities|FlowControl|Delay 1e+01)
      (Class|AISenseHearing|ReportNoiseEvent (Transformation|GetActorLocation) 1e+03 self 0.0 "None")
      (Development|PrintString "Made Noise"))))

(event EventTick
  (params (DeltaSeconds :type Float%20%28single-precision%29)))

(fn ConstructionScript)

(fn CastChecker
  (params (Object :type Actor%20Object%20Reference) (Exit? :type Boolean))
  (Variables|Default|SetOther%20Actor Object)
  (if (or (.bSuccess (Utilities|Casting|CastToBP_Sagar Object)) (.bSuccess (Utilities|Casting|CastToBP_Nandini_Pawn Object)))
    (if Exit?
      (Variables|Default|SetOther%20Actor 0)
      (return false)
      (else
        (return true)))
    (else
      (Variables|Default|SetOther%20Actor 0))))

(fn GetInteractableName
  (return "Rice Cooker"))