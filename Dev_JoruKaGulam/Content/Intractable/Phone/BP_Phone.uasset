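; BP_Phone is an interactable phone actor whose screen cycles through a set of camera materials.
; PhoneInteract takes a left or right input and steps CurrentActiveCamera through the CameraMats array, wrapping at both ends.
; It then applies the selected material to slot 1 of the phone body mesh and prints the new index for debugging.
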(event EventBeginPlay)

(event Collision|EventActorBeginOverlap
  (params (OtherActor :type Actor%20Object%20Reference)))

(event EventTick
  (params (DeltaSeconds :type Float%20%28single-precision%29)))

(fn ConstructionScript)

(fn PhoneInteract
  (params (Interact%20Input :type E_Phone_Interact%20Enum :default "NewEnumerator0"))
  (bind _camera_mats (Variables|Default|GetCamera%20Mats))
  (bind _returnvalue (Utilities|Array|Length _camera_mats))
  (bind _returnvalue_2 (- _returnvalue 1))
  (switch Utilities|FlowControl|Switch|SwitchonE_Phone_Interact Interact%20Input
    (:NewEnumerator0
      (if (<= (Variables|Default|GetCurrent%20Active%20Camera) 0)
        (Variables|Default|SetCurrent%20Active%20Camera _returnvalue_2)
        (else
          (Math|Integer|DecrementInt (Variables|Default|GetCurrent%20Active%20Camera)
            (:%20%20
              _)))))
    (:NewEnumerator1
      (if (>= (Variables|Default|GetCurrent%20Active%20Camera) _returnvalue_2)
        (Variables|Default|SetCurrent%20Active%20Camera 0)
        (else
          (Math|Integer|IncrementInt (Variables|Default|GetCurrent%20Active%20Camera)
            (:%20%20
              _))))))
  (Rendering|Material|SetMaterial (Variables|Default|GetCellPhone_PhoneBody) 1 (Utilities|Array|Get(acopy) (Variables|Default|GetCamera%20Mats) (Variables|Default|GetCurrent%20Active%20Camera)))
  (Development|PrintString (Utilities|String|Append "Camera index changed to : " (Utilities|String|ToString(Integer) (Variables|Default|GetCurrent%20Active%20Camera))))
  (return))