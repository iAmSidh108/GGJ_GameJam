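; BP_Landline is a landline phone that rings and emits loud noise events until it is picked up.
; Ring loops on a delay, replaying the audio and reporting noise at the phone's location, which AI hearing can detect.
; An actor tagged "Nandhini" overlapping the Box triggers PhonePickup, which stops the audio and sets the flag that ends the loop.
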(event OnComponentBeginOverlap(Box)
  (params (OverlappedComponent :type Primitive%20Component%20Object%20Reference) (OtherActor :type Actor%20Object%20Reference) (OtherComp :type Primitive%20Component%20Object%20Reference) (OtherBodyIndex :type Integer) (bFromSweep :type Boolean) (SweepResult :type Hit%20Result%20Structure%20%28by%20ref%29))
  (if (Actor|ActorHasTag OtherActor "Nandhini")
    (CallFunction|PhonePickup)))

(event Custom|Ring
  (Variables|Default|SetPhone%20Answered false)
  (Audio|Components|Audio|Play (Variables|Default|GetAudio) 0.0 :!label _label)
  (Class|AISenseHearing|ReportNoiseEvent (Transformation|GetActorLocation) 1e+03 self 0.0 "None")
  (Utilities|FlowControl|Delay 4.0)
  (if (not (Variables|Default|GetPhone%20Answered))
    (goto _label)))

(event Custom|Phone%20Pickup
  (Variables|Default|SetPhone%20Answered true)
  (Audio|Components|Audio|Stop (Variables|Default|GetAudio)))

(event EventBeginPlay)

(event Collision|EventActorBeginOverlap
  (params (OtherActor :type Actor%20Object%20Reference)))

(event EventTick
  (params (DeltaSeconds :type Float%20%28single-precision%29)))

(fn ConstructionScript)