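; BP_Key is a key pickup that counts as a completed task when collected.
; Box overlap with BP_Sagar or BP_Nandini_Pawn toggles the mesh's custom depth highlight and an interaction prompt.
; Tick re-enables mesh physics and polls PickUpPressed, which only works for BP_Sagar.
; A pickup plays a Timeline that lifts the mesh, then calls TaskCompleted on JOG_GM and destroys the actor.
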(event OnComponentBeginOverlap(Box)
  (params (OverlappedComponent :type Primitive%20Component%20Object%20Reference) (OtherActor :type Actor%20Object%20Reference) (OtherComp :type Primitive%20Component%20Object%20Reference) (OtherBodyIndex :type Integer) (bFromSweep :type Boolean) (SweepResult :type Hit%20Result%20Structure%20%28by%20ref%29))
  (Variables|Default|SetCan%20interact? (CallFunction|CastChecker OtherActor false))
  (Rendering|SetRenderCustomDepth (Variables|Default|GetMesh) (Variables|Default|GetCan%20interact?))
  (Rendering|SetVisibility (Variables|Default|GetInteraction) (Variables|Default|GetCan%20interact?) false))

(event OnComponentEndOverlap(Box)
  (params (OverlappedComponent :type Primitive%20Component%20Object%20Reference) (OtherActor :type Actor%20Object%20Reference) (OtherComp :type Primitive%20Component%20Object%20Reference) (OtherBodyIndex :type Integer))
  (Variables|Default|SetCan%20interact? (CallFunction|CastChecker OtherActor true))
  (Rendering|SetRenderCustomDepth (Variables|Default|GetMesh) (Variables|Default|GetCan%20interact?))
  (Rendering|SetVisibility (Variables|Default|GetInteraction) (Variables|Default|GetCan%20interact?) false))

(event EventTick
  (params (DeltaSeconds :type Float%20%28single-precision%29))
  (bind _other_actor (Variables|Default|GetOther%20Actor))
  (Physics|SetSimulatePhysics (Variables|Default|GetMesh) true)
  (Utilities|IsValid _other_actor
    (:Is%20Valid
      (if (Variables|/Game/Game_Files/Player/BP_Sagar.BP_Sagar_C|GetPickUpPressed (.AsBP%20Sagar (Utilities|Casting|CastToBP_Sagar _other_actor)))
        (Variables|Default|SetLoc (Transformation|GetActorLocation))
        (if true
          (bind _newtrack_0 (Timeline|Timeline Play)
            (:Update
              (Transformation|SetWorldLocation (Variables|Default|GetMesh) (Math|Vector|MakeVector (.x (Variables|Default|GetLoc)) (.y (Variables|Default|GetLoc)) (+ (.z (Variables|Default|GetLoc)) (Math|Float|Lerp 0.0 1e+02 _newtrack_0))) false false))
            (:Finished
              (Default|TaskCompleted (.AsJOG%20GM (Utilities|Casting|CastToJOG_GM (Game|GetGameMode))))
              (Actor|DestroyActor))))))))

(fn ConstructionScript)

(fn CastChecker
  (params (Object :type Actor%20Object%20Reference) (Exit? :type Boolean))
  (Variables|Default|SetOther%20Actor Object)
  (if (or (.bSuccess (Utilities|Casting|CastToBP_Sagar Object)) (.bSuccess (Utilities|Casting|CastToBP_Nandini_Pawn Object)))
    (if Exit?
      (Variables|Default|SetOther%20Actor 0)
      (return false)
      (else
        (return true)))
    (else
      (Variables|Default|SetOther%20Actor 0))))