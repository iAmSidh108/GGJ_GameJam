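; Interactable wallet pickup that serves as a task objective in one specific level of the JOG game mode.
; The mesh simulates physics, and querying its interactable name also triggers a five-second custom-depth glow.
; Interacting during that level plays a timeline that raises the mesh, then reports task completion to the game mode and destroys the actor.
; A helper tracks whether the other actor is a Sagar or Nandini pawn.
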(event Custom|Enable%20Glow%20for%205%20Seconds
  (Rendering|SetRenderCustomDepth (Variables|Default|GetMesh) true)
  (Utilities|FlowControl|Delay 5.0)
  (Rendering|SetRenderCustomDepth (Variables|Default|GetMesh) false))

(event EventTryInteract
  (params (Actor%20 :type Actor%20Object%20Reference))
  (Variables|Default|SetLoc (Transformation|GetActorLocation))
  (if (Utilities|Enum|Equal(Enum) (Variables|/Game/Game_Files/JOG_GM.JOG_GM_C|GetCurrent%20Level (.AsJOG%20GM (Utilities|Casting|CastToJOG_GM (Game|GetGameMode)))) "NewEnumerator5")
    (bind _newtrack_0 (Timeline|Timeline Play)
      (:Update
        (Transformation|SetWorldLocation (Variables|Default|GetMesh) (Math|Vector|MakeVector (.x (Variables|Default|GetLoc)) (.y (Variables|Default|GetLoc)) (+ (.z (Variables|Default|GetLoc)) (Math|Float|Lerp 0.0 1e+02 _newtrack_0))) false false))
      (:Finished
        (Default|TaskCompleted (.AsJOG%20GM (Utilities|Casting|CastToJOG_GM (Game|GetGameMode))))
        (Actor|DestroyActor)))))

(event EventBeginPlay
  (Physics|SetSimulatePhysics (Variables|Default|GetMesh) true))

(fn ConstructionScript)

(fn CastChecker
  (params (Object :type Actor%20Object%20Reference) (Exit? :type Boolean))
  (Variables|Default|SetOther%20Actor Object)
  (if (or (.bSuccess (Utilities|Casting|CastToBP_Sagar Object)) (.bSuccess (Utilities|Casting|CastToBP_Nandini_Pawn Object)))
    (if Exit?
      (Variables|Default|SetOther%20Actor 0)
      (return false)
      (else
        (return true)))
    (else
      (Variables|Default|SetOther%20Actor 0))))

(fn GetInteractableName
  (CallFunction|EnableGlowfor5Seconds)
  (return "Wallet"))